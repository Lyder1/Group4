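; BP_Goal is a level goal object that triggers the win screen when the archer reaches it.
; Its Box overlap sets a Won flag when the overlapping actor matches ArcherReference, and BeginPlay clears that flag.
; Tick polls the flag, creating a win-screen widget, showing the mouse cursor and switching input to UI-only.
; Won is never reset after a win, so a new widget is added every frame.
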(event `self.ReceiveBeginPlay`
  (set `self.Won` false))

(event `self.ReceiveTick`
  (params (DeltaSeconds :type "Float (single-precision)"))
  (bind _returnvalue (`GameplayStatics.GetPlayerController` 0))
  (bind _goal_reference (`self.Goal Reference`))
  (if (`self.Won`)
    (bind _returnvalue_2 (`|CreateWidget` "/Game/Blueprints/User_Interface/WB_WinScreen.WB_WinScreen_C"))
    (set `self.Goal Reference` _returnvalue_2)
    (set `PlayerController.bShowMouseCursor` true _returnvalue)
    (`WidgetBlueprintLibrary.SetInputMode_UIOnlyEx` _returnvalue _goal_reference)
    (`UserWidget.AddToViewport` _goal_reference 2)))

(event `self.Box.OnComponentBeginOverlap`
  (params (OverlappedComponent :type "PrimitiveComponent Object Reference") (OtherActor :type "Actor Object Reference") (OtherComp :type "PrimitiveComponent Object Reference") (OtherBodyIndex :type Integer) (bFromSweep :type Boolean) (SweepResult :type "HitResult Structure (by ref)"))
  (if (== OtherActor (`self.Archer Reference`))
    (set `self.Won` true)))

(fn `UserConstructionScript`)