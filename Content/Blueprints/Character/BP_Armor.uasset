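; BP_Armor is an armor actor with a floating health bar driven by its current and maximum health.
; The bar's widget component starts hidden at BeginPlay and is revealed from Tick once health is below maximum.
; While damaged, Tick writes the health ratio to the WB_EnemyHealthBar progress bar and rotates the component toward the player camera.
; The graph shows no damage handling and never hides the bar again.
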(event `self.ReceiveBeginPlay`
  (`SceneComponent.SetHiddenInGame` (`self.HealthBarWidget`) true false))

(event `self.ReceiveTick`
  (params (DeltaSeconds :type "Float (single-precision)"))
  (bind _healthbarwidget (`self.HealthBarWidget`))
  (bind _aswb_enemy_health_bar (cast `/Game/Blueprints/User_Interface/WB_EnemyHealthBar` (`WidgetComponent.GetWidget` (`self.HealthBarWidget`))))
  (if (< (`self.CurrentHealth`) (`self.MaxHealth`))
    (`SceneComponent.SetHiddenInGame` (`self.HealthBarWidget`) false false)
    (`ProgressBar.SetPercent` (`/Game/Blueprints/User_Interface/WB_EnemyHealthBar.HealthBar` _aswb_enemy_health_bar) (/ (`self.CurrentHealth`) (`self.MaxHealth`)))
    (`SceneComponent.K2_SetWorldRotation` _healthbarwidget (`KismetMathLibrary.FindLookAtRotation` (`SceneComponent.K2_GetComponentLocation` _healthbarwidget) (`SceneComponent.K2_GetComponentLocation` (`PlayerCameraManager.TransformComponent` (`GameplayStatics.GetPlayerCameraManager` 0)))) false false)))

(fn `UserConstructionScript`)