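; BP_Archer is an archer Blueprint with rudimentary health and ammo handling driven by hard-coded keys.
; R refills Ammo, H restores Health to its maximum and F subtracts Health, with both health keys printing the new value.
; Unconnected nodes hold HUD widget creation, ammo consumption and edits to a separate Playerhealth variable, so none of these run.
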(event `Key|R`
  (params (Key :type "Key Structure"))
  (:`Pressed`
    (set `self.Ammo` 10)))

(event `Key|H`
  (params (Key :type "Key Structure"))
  (:`Pressed`
    (bind _output_get (set `self.Health` (`self.MaxHealth_0`)))
    (`KismetSystemLibrary.PrintString` (`KismetStringLibrary.Conv_DoubleToString` _output_get))))

(event `Key|F`
  (params (Key :type "Key Structure"))
  ;[1 1 1] Health count
  (:`Pressed`
    (bind _output_get (set `self.Health` (- (`self.Health`) 1.0)))
    (`KismetSystemLibrary.PrintString` (`KismetStringLibrary.Conv_DoubleToString` _output_get))))

(event `Key|LeftMouseButton`
  (params (Key :type "Key Structure"))
  ;[1 1 1] Ammo count
)

(event `self.ReceiveBeginPlay`)

(fn `UserConstructionScript`)